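; Something_BP is a collectible item that responds to the OnInteract event.
; If ItemCollected is false, it calls the parent interaction, plays a pickup sound at the actor's location, hides the Item component and disables collision on Item and Trigger.
; The flag is only read here, and the actor is hidden in place with no destroy call.
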(event `self.OnInteract`
  (if (not (`self.bItemCollected`))
    (`parent.OnInteract`)
    (`GameplayStatics.PlaySoundAtLocation` "/Game/Assets/Audio/pickup.pickup" (`self.K2_GetActorLocation`) (struct) 1.0 1.0 0.0 null null null)
    (`SceneComponent.SetVisibility` (`self.Item`) false false)
    (`PrimitiveComponent.SetCollisionEnabled` (`self.Item`) "NoCollision")
    (`PrimitiveComponent.SetCollisionEnabled` (`self.trigger`) "NoCollision")))

(fn `UserConstructionScript`)
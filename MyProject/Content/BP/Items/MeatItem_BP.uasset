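; MeatItem_BP is an interactable meat pickup item that extends a parent item Blueprint.
; On interact, if ItemCollected is false, it runs the parent's OnInteract and plays a pickup sound at its location.
; It then hides the Item component and disables collision on both Item and Trigger, leaving the actor in the world rather than destroying it.
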(event `self.OnInteract`
  (if (not (`self.bItemCollected`))
    (`parent.OnInteract`)
    (`GameplayStatics.PlaySoundAtLocation` "/Game/Assets/Audio/pickup.pickup" (`self.K2_GetActorLocation`) (struct) 1.0 1.0 0.0 null null null)
    (`SceneComponent.SetVisibility` (`self.Item`) false false)
    (`PrimitiveComponent.SetCollisionEnabled` (`self.Item`) "NoCollision")
    (`PrimitiveComponent.SetCollisionEnabled` (`self.trigger`) "NoCollision")))

(fn `UserConstructionScript`)
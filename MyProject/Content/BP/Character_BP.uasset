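; Player character Blueprint that acts as the UI layer for dialogue, quests and inventory, with cheat keys on 1–4.
; BeginPlay creates the quest list and a hidden inventory widget, which OnRefreshInventory shows and fills from EquipmentInventory.
; OnShowUI spawns a player widget on demand with Game-and-UI input, quest events push info and completion messages to it, and OnHideUI releases it.
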(event `self.OnShowUI`
  (params (characterName :type Name))
  (bind _returnvalue (`GameplayStatics.GetPlayerController` 0))
  (if (not (`KismetSystemLibrary.IsValid` (`self.PlayerUI`)))
    (bind _returnvalue_2 (`|CreateWidget` "/Game/BP/UI/PlayerUI_BP.PlayerUI_BP_C" _returnvalue))
    (`WidgetBlueprintLibrary.SetInputMode_GameAndUIEx` _returnvalue _returnvalue_2 "LockAlways")
    (`UserWidget.AddToViewport` _returnvalue_2 0)
    (bind _output_get (set `self.PlayerUI` _returnvalue_2))
    (`/Game/BP/UI/PlayerUI_BP.ShowUI` _output_get (`KismetTextLibrary.Conv_NameToText` characterName))))

(event `self.OnHideUI`
  (bind _playerui (`self.PlayerUI`))
  (if (`KismetSystemLibrary.IsValid` _playerui)
    (`UINavWidget.ReturnToParent` _playerui false 0)
    (set `self.PlayerUI` null)))

(event `Key|One`
  (params (Key :type "Key Structure"))
  ;[1 1 1] Cheat Code
  (:`Pressed`
    (`self.CheatGrape`)))

(event `Key|Three`
  (params (Key :type "Key Structure"))
  ;[1 1 1] Cheat Code
  (:`Pressed`
    (`self.CheatHay`)))

(event `Key|Two`
  (params (Key :type "Key Structure"))
  ;[1 1 1] Cheat Code
  (:`Pressed`
    (`self.CheatMeat`)))

(event `Key|Four`
  (params (Key :type "Key Structure"))
  ;[1 1 1] Cheat Code
  (:`Pressed`
    (`self.CheatSomething`)))

(event `self.OnShowQuestInfo`
  (params (Quest :type "Quest Structure"))
  (bind (_charactername _questid _message _sortdescription _completemessage _itemid _itemquesttexture) (break `Quest` Quest))
  (bind _playerui (`self.PlayerUI`))
  ;[1 1 1] Show Quest Info
  (if (`KismetSystemLibrary.IsValid` _playerui)
    (`/Game/BP/UI/PlayerUI_BP.ShowQuestInfo` _playerui _message _itemquesttexture)))

(event `self.OnShowQuestCompleted`
  (params (message :type "Text (by ref)"))
  (bind _playerui (`self.PlayerUI`))
  ;[1 1 1] Show Quest Completed
  (if (`KismetSystemLibrary.IsValid` _playerui)
    (`/Game/BP/UI/PlayerUI_BP.ShowQuestCompleted` _playerui message)))

(event `self.OnShowUpdatedQuestList`
  (params (questTextList :type "Array of Text (by ref)"))
  (bind _questui (`self.QuestUI`))
  ;[1 1 1] Quest
  (if (`KismetSystemLibrary.IsValid` _questui)
    (`/Game/BP/UI/QuestUI_BP.UpdateQuestList` _questui questTextList)))

(event `self.ReceiveBeginPlay`
  ;[1 1 1] Initialization
  (bind _returnvalue (`|CreateWidget` "/Game/BP/UI/QuestUI_BP.QuestUI_BP_C" (`GameplayStatics.GetPlayerController` 0)))
  (`UserWidget.AddToViewport` _returnvalue 0)
  (set `self.QuestUI` _returnvalue)
  (bind _returnvalue_2 (`|CreateWidget` "/Game/BP/UI/InventoryUI_BP.InventoryUI_BP_C"))
  (bind _output_get (set `self.InventoryUI` _returnvalue_2))
  (`UserWidget.AddToViewport` _output_get 0)
  (`/Game/BP/UI/InventoryUI_BP.Hide` _output_get))

(event `self.OnRefreshInventory`
  (bind _inventoryui (`self.InventoryUI`))
  ;[1 1 1] OnRefreshInventory
  (if (`KismetSystemLibrary.IsValid` _inventoryui)
    (`/Game/BP/UI/InventoryUI_BP.Show` _inventoryui)
    (`/Game/BP/UI/InventoryUI_BP.Refresh Inventory` _inventoryui (`self.equipmentInventory`))))

(fn `UserConstructionScript`
  (`parent.UserConstructionScript`))
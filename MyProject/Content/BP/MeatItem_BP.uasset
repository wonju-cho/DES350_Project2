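; MeatItem_BP is a collectible meat item that responds to interaction.
; OnInteract only acts while ItemCollected is false: it calls the parent's OnInteract, plays a click sound at the actor's location, then hides the Item component.
; The nodes that would disable collision on Item and Trigger are unconnected and never run.
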(event `self.OnInteract`
  (if (not (`self.bItemCollected`))
    (`parent.OnInteract`)
    (`GameplayStatics.PlaySoundAtLocation` "/Engine/VREditor/Sounds/UI/Click_on_Button.Click_on_Button" (`self.K2_GetActorLocation`) (struct) 1.0 1.0 0.0 null null null)
    (`SceneComponent.SetVisibility` (`self.Item`) false false)))

(fn `UserConstructionScript`)